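; Oceanology infinite-ocean actor that builds its water surface as a procedural instanced-mesh quadtree grid, skipped on dedicated servers.
; Construction lays out the grid, scales the far ocean mesh and underlying post-process volume from the QuadTree settings, and toggles ocean visibility.
; Caustics height is written to MPC_Ocean at construction and BeginPlay.
; Dedicated servers accept QuadTree updates, and its RepNotify rebuilds the structure.
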(event Custom|Add%20Caustics
  ;[0 0 0] Caustics
  (|Caustics))

(event Custom|SetUpdateQuadTreeServer
  (params (Quad%20Tree :type Quad%20Tree%20INF%20Structure))
  ;[0 0 0] Quadtree
  (CallFunction|UpdateQuadTree Quad%20Tree))

(event Custom|Add%20Quadtree
  ;[0 0 0] Quadtree
  (|Quadtree))

(event EventBeginPlay
  (|CallParentFunction)
  ;[0 0 0] Caustics in simulation mode
  (CallFunction|AddCaustics))

(event EventTick
  (params (DeltaSeconds :type Float%20%28single-precision%29)))

(fn ConstructionScript
  (|CallParentFunction)
  (CallFunction|Structure))

(fn OnRepQuadTree
  (CallFunction|Structure))

(fn Structure
  (bind _quad_tree (Variables|QuadTree|GetQuad%20Tree))
  (bind _islandandocean (Utilities|Struct|BreakQuadTree_INF _quad_tree))
  (bind _returnvalue (/ _islandandocean 6e+01))
  (bind _returnvalue_2 (Math|Conversions|ToVector(Float) _returnvalue))
  ;[0 0 0] Quadtree
  (CallFunction|AddQuadtree)
  ;[0 0 0] Caustics
  (CallFunction|AddCaustics)
  ;[0 0 0] Scale And Location
  (Transformation|SetWorldScale3D (Variables|Default|GetPostProcess%20Volume) (Math|Vector|MakeVector (.x _returnvalue_2) (.y _returnvalue_2) 3e+03))
  (Transformation|AddLocalOffset (Variables|Default|GetPostProcess%20Volume) (Math|Vector|MakeVector 0.0 0.0 -9e+04) false false)
  (Transformation|SetWorldScale3D (Variables|Default|GetFarOceanMesh) (Math|Conversions|ToVector(Float) (/ (- (Utilities|Struct|BreakQuadTree_INF (Variables|QuadTree|GetQuad%20Tree)) (Math|Float|MakeLiteralFloat 1024.0)) 256.0))))

(fn UpdateQuadTree
  (params (Quad%20Tree%20INF :type Quad%20Tree%20INF%20Structure))
  (if (Networking|IsDedicatedServer)
    (Variables|QuadTree|SetQuad%20Tree Quad%20Tree%20INF)))